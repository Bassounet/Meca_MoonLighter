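; BP_TourelleFix is a turret that fires projectiles automatically on a repeating timer.
; On BeginPlay, if CanFire is true, it starts a looping timer at the TimeForFire interval, with a random initial delay, and stores the handle in REFTimer.
; Each tick of that timer spawns a BP_Projectile at component R's transform and plays a world camera shake from that location.
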(event `self.ReceiveBeginPlay`
  ;[1 1 1] Make Ref
  (`self.Fire`))

(event `Fire`
  ;[1 1 1] Fire
  (if (`self.CanFire`)
    (bind _returnvalue (`KismetSystemLibrary.K2_SetTimerDelegate` (delegate `Faya`) (`self.TimeForFire`) true (`KismetMathLibrary.RandomFloatInRange` 0.2 1.0)))
    (set `self.REF_Timer` _returnvalue)))

(event `Faya`
  ;[1 1 1] Fire
  (`|SpawnActorFromClass` "/Game/PureBP/BP_Projectile.BP_Projectile_C" (`SceneComponent.K2_GetComponentToWorld` (`self.r`)) "Undefined" "OverrideRootScale" null null)
  (`GameplayStatics.PlayWorldCameraShake` "/Game/PureBP/BP_CamShake.BP_CamShake_C" (`SceneComponent.K2_GetComponentLocation` (`self.r`)) 10000.0))

(fn `UserConstructionScript`)