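; BP_Projectile is a projectile actor that hurts the player's TopDownCharacter on overlap.
; Each tick it rotates its root component in world space to face player 0's character.
; When component F begins an overlap, it casts the other actor to TopDownCharacter and calls Hurted unless that character's Invulerable flag is set.
; The graphs contain no movement or destroy logic.
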(event `self.ReceiveTick`
  (params (DeltaSeconds :type "Float (single-precision)"))
  ;[1 1 1] Look at player
  (`SceneComponent.K2_SetWorldRotation` (`self.DefaultSceneRoot`) (`KismetMathLibrary.FindLookAtRotation` (`SceneComponent.K2_GetComponentLocation` (`self.DefaultSceneRoot`)) (`self.K2_GetActorLocation` (`GameplayStatics.GetPlayerCharacter` 0))) false false))

(event `self.f.OnComponentBeginOverlap`
  (params (OverlappedComponent :type "PrimitiveComponent Object Reference") (OtherActor :type "Actor Object Reference") (OtherComp :type "PrimitiveComponent Object Reference") (OtherBodyIndex :type Integer) (bFromSweep :type Boolean) (SweepResult :type "HitResult Structure (by ref)"))
  (bind _astop_down_character (cast `/Game/TopDownBP/Blueprints/TopDownCharacter` OtherActor))
  (if (not (`/Game/TopDownBP/Blueprints/TopDownCharacter.Invulerable` _astop_down_character))
    (`/Game/TopDownBP/Blueprints/TopDownCharacter.Hurted` _astop_down_character)))

(fn `UserConstructionScript`)