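; Teleporter-style trigger actor that swaps levels when the TopDownCharacter enters its box, with a flickering point light.
; On overlap it loads LevelToLoad as a dynamic level instance, then requests a non-blocking unload of LevelToUnLoad.
; From BeginPlay, Clignotage loops a delay and a timeline that lerps the light's current intensity toward a random value, resetting the play rate from Duration after each pass.
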(event `self.ReceiveBeginPlay`
  (`self.Clignotage`))

(event `Clignotage`
  (`KismetSystemLibrary.RetriggerableDelay` (`self.Duration`) :!label _label)
  (set `self.MaxLight` (`KismetMathLibrary.RandomFloatInRange` 5766.254883 66758.476562))
  (bind (_direction _newtrack_0) (`Timeline|A` :`NewTime` 10.0 :!via `PlayFromStart`)
    (:`Update`
      (`LightComponent.SetIntensity` (`self.PointLight`) (`KismetMathLibrary.Lerp` (`LightComponentBase.Intensity` (`self.PointLight`)) (`self.MaxLight`) _newtrack_0)))
    (:`Finished`
      (`TimelineComponent.SetPlayRate` (`self.A`) (/ 1.0 (`self.Duration`)))
      (goto _label))))

(event `self.Box.OnComponentBeginOverlap`
  (params (OverlappedComponent :type "PrimitiveComponent Object Reference") (OtherActor :type "Actor Object Reference") (OtherComp :type "PrimitiveComponent Object Reference") (OtherBodyIndex :type Integer) (bFromSweep :type Boolean) (SweepResult :type "HitResult Structure (by ref)"))
  (cast `/Game/TopDownBP/Blueprints/TopDownCharacter` OtherActor)
  (`|ExecutionSequence`
    (:`then_0`
      (`LevelStreamingDynamic.LoadLevelInstanceBySoftObjectPtr` (`self.LevelToLoad`) (0.0 0.0 0.0) (struct) "" "/Script/Engine.LevelStreamingDynamic"))
    (:`then_1`
      (`GameplayStatics.UnloadStreamLevelBySoftObjectPtr` (`self.LevelToUnLoad`)))))

(fn `UserConstructionScript`)